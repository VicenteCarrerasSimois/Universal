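; BP_Personaje1 is the player character for a side-scrolling game, moving along the X axis and jumping through Enhanced Input.
; Movement flips the controller yaw according to the sign of acceleration to face the travel direction.
; Interface-style events subtract damage from health and add collected coins to a printed counter.
; Tick polls health, and when it drops below zero the character moves to a hardcoded respawn location with full health.
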(event `self.ReceiveTick`
  (params (DeltaSeconds :type "Float (single-precision)"))
  (`self.ChequeoVida`))

(event `self.ReceiveBeginPlay`
  (bind _asplayer_controller (cast `PlayerController` (`self.GetController`)))
  (`EnhancedInputSubsystemInterface.AddMappingContext` (pcsubsystem `EnhancedInputLocalPlayerSubsystem` _asplayer_controller) "/Game/BP_Personaje/Mapping/IMC_Personaje.IMC_Personaje" 0 (struct))
  (bind _output_get (set `self.Vida` (`self.VidaMaxima`)))
  (`KismetSystemLibrary.PrintString` (`KismetStringLibrary.Conv_DoubleToString` _output_get)))

(event `EnhancedInput|/Game/BP_Personaje/Mapping/Inputs/IA_Movimiento`
  (params (ActionValue :type "Float (double-precision)") (ElapsedSeconds :type "Float (double-precision)") (TriggeredSeconds :type "Float (double-precision)") (InputAction :type "InputAction Object Reference" :default "/Game/BP_Personaje/Mapping/Inputs/IA_Movimiento.IA_Movimiento"))
  (bind _returnvalue (`self.GetController`))
  (bind _returnvalue_x (`KismetMathLibrary.BreakVector` (`CharacterMovementComponent.GetCurrentAcceleration` (`self.CharacterMovement`))))
  ;[1 1 1] Caminar/Movimiento
  (:`Triggered`
    (`self.AddMovementInput` (1.0 0.0 0.0) ActionValue)
    (`/Engine/EditorBlueprintResources/StandardMacros.CompareFloat` _returnvalue_x
      (:`>`
        (`Controller.SetControlRotation` _returnvalue (`KismetMathLibrary.MakeRotator` 0.0)))
      (:`<`
        (`Controller.SetControlRotation` _returnvalue (`KismetMathLibrary.MakeRotator` 0.0 0.0 180.0))))))

(event `EnhancedInput|/Game/BP_Personaje/Mapping/Inputs/IA_Salto`
  (params (ActionValue :type Boolean) (ElapsedSeconds :type "Float (double-precision)") (TriggeredSeconds :type "Float (double-precision)") (InputAction :type "InputAction Object Reference" :default "/Game/BP_Personaje/Mapping/Inputs/IA_Salto.IA_Salto"))
  ;[0.3894 1 0.09903] Salto
  (:`Started`
    (`self.Jump`))
  (:`Completed`
    (`self.StopJumping`)))

(event `/Game/Enemigo/BPI_Enemigo.BPI_Daño`
  (params (`Daño` :type "Float (double-precision)"))
  (`self.MequitaVidaNashei` `Daño`))

(event `/Game/Atomoneda/BPI_Moneda.Moneda`
  (params (ConseguirMoneda :type Integer))
  ;[1 0.8859 0.1768] Monedita Section
  (bind _output_get (set `self.MonedaNashei` (+ ConseguirMoneda (`self.MonedaNashei`))))
  (`KismetSystemLibrary.PrintString` (`KismetStringLibrary.Concat_StrStr` (`KismetStringLibrary.Conv_IntToString` _output_get)) true true (struct :`R` 1.0 :`B` 0.418581 :`A` 1.0) 3.0))

(fn `ChequeoVida`
  (if (< (`self.Vida`) 0.0)
    (`KismetSystemLibrary.PrintString` "Skill Issue?")
    (`self.K2_SetActorLocation` (128.0 0.0 -630.0))
    (set `self.Vida` (`self.VidaMaxima`))))

(fn `MequitaVidaNashei`
  (params (Damage :type "Float (double-precision)"))
  (set `self.Vida` (- (`self.Vida`) Damage)))

(fn `UserConstructionScript`)